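; Longsword weapon Blueprint that generates a procedural swish sound as the blade moves, using a modular synth component.
; On BeginPlay it loads a monophonic noise-oscillator preset into SwishSynth and starts a sustained note.
; Each Tick it reads the speed of the WeaponHead component, feeding it directly into the filter frequency and, scaled down, into both oscillator gains, so faster swings sound brighter and louder.
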(event EventBeginPlay
  (Class|ModularSynthComponent|SetSynthPreset (Variables|Default|Getswish_synth) (Utilities|Struct|MakeModularSynthPreset false "Noise" 1.0 0.0 0.0 0.0 0.5 "Noise" 1.0 0.0 0.0 2.5 0.5 0.0 false false 0.5 0.0 1.0 0.0 "Sine" "Sync" "PatchToNone" 1.0 0.0 "Sine" "Sync" "PatchToNone" -3.0 1e+01 1e+02 0.707 5e+03 "PatchToNone" "PatchToNone" false false 1.0 1e+01 1e+02 0.707 5e+03 true false 8e+03 2.0 "LowPass" "Ladder" false "PingPong" 7e+02 0.7 0.3 0.2 false 0.2 0.5 2.0 (Utilities|Array|MakeArray "")))
  (Class|ModularSynthComponent|Noteon (Variables|Default|Getswish_synth) 0.0 127 -1.0))

(event EventTick
  (params (DeltaSeconds :type Float%20%28single-precision%29))
  (bind _swish_synth (Variables|Default|Getswish_synth))
  (bind _weapon_head (Variables|Default|Getweapon_head))
  (bind _returnvalue (Transformation|GetComponentVelocity _weapon_head))
  (bind _returnvalue_2 (Math|Vector|VectorLength _returnvalue))
  (bind _returnvalue_3 (/ _returnvalue_2 5e+03))
  (Class|ModularSynthComponent|SetFilterFrequency (Variables|Default|Getswish_synth) _returnvalue_2)
  (Class|ModularSynthComponent|SetOscGain _swish_synth 0 _returnvalue_3)
  (Class|ModularSynthComponent|SetOscGain _swish_synth 1 _returnvalue_3))

(fn ConstructionScript)